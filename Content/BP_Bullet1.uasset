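; BP_Bullet1 is a projectile that kills enemies and credits the player for each one.
; Sphere overlap with an Enemy, given a valid Player reference, increments Score and Kill, pushes both through their ScoreRef and KillRef references, then destroys bullet and enemy.
; Overlapping a BP_Tunnel or HealthPack destroys only the bullet, as does a blocking hit on a tunnel.
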(event OnComponentBeginOverlap(Sphere)
  (params (OverlappedComponent :type Primitive%20Component%20Object%20Reference) (OtherActor :type Actor%20Object%20Reference) (OtherComp :type Primitive%20Component%20Object%20Reference) (OtherBodyIndex :type Integer) (bFromSweep :type Boolean) (SweepResult :type Hit%20Result%20Structure%20%28by%20ref%29))
  (bind _player (Variables|Default|GetPlayer))
  (Utilities|Casting|CastToBP_Tunnel OtherActor
    (:then
      (Actor|DestroyActor))
    (:CastFailed
      (bind _asenemy (Utilities|Casting|CastToEnemy OtherActor)
        (:then
          (Utilities|IsValid _player
            (:Is%20Valid
              (bind _output_get (Variables|/Game/InfiniteMatrix/Blueprints/BP_Player.BP_Player_C|SetScore _player (+ (Variables|/Game/InfiniteMatrix/Blueprints/BP_Player.BP_Player_C|GetScore _player) 1)))
              (Default|UpdateScore (Variables|/Game/InfiniteMatrix/Blueprints/BP_Player.BP_Player_C|GetScoreRef _player) _output_get)
              (Variables|/Game/InfiniteMatrix/Blueprints/BP_Player.BP_Player_C|SetKill _player (+ (Variables|/Game/InfiniteMatrix/Blueprints/BP_Player.BP_Player_C|GetKill _player) 1))
              (Default|UpdateScore (Variables|/Game/InfiniteMatrix/Blueprints/BP_Player.BP_Player_C|GetKillRef _player) (Variables|/Game/InfiniteMatrix/Blueprints/BP_Player.BP_Player_C|GetKill _player))
              (Actor|DestroyActor)
              (Actor|DestroyActor _asenemy))))
        (:CastFailed
          (Utilities|Casting|CastToHealthPack OtherActor)
          (Actor|DestroyActor))))))

(event OnComponentHit(Sphere)
  (params (HitComponent :type Primitive%20Component%20Object%20Reference) (OtherActor :type Actor%20Object%20Reference) (OtherComp :type Primitive%20Component%20Object%20Reference) (NormalImpulse :type Vector :default "0, 0, 0") (Hit :type Hit%20Result%20Structure%20%28by%20ref%29))
  (Utilities|Casting|CastToBP_Tunnel OtherActor)
  (Actor|DestroyActor))

(event EventBeginPlay)

(event Collision|EventActorBeginOverlap
  (params (OtherActor :type Actor%20Object%20Reference)))

(event EventTick
  (params (DeltaSeconds :type Float%20%28single-precision%29)))

(fn ConstructionScript)